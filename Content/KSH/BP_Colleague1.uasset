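; BP_Colleague1 is a colleague actor that reacts once the player comes within its sphere trigger.
; Its widget stays hidden from BeginPlay until an overlap by a Player-tagged actor reveals it, loops an RPG hero idle animation and turns the colleague toward the player pawn.
; The same overlap sets a short lifespan so the actor destroys itself, then calls StartGod on the overlapping JamCharacter.
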(event `self.ReceiveBeginPlay`
  (`SceneComponent.SetVisibility` (`self.Widget`) false false))

(event `self.Sphere.OnComponentBeginOverlap`
  (params (OverlappedComponent :type "PrimitiveComponent Object Reference") (OtherActor :type "Actor Object Reference") (OtherComp :type "PrimitiveComponent Object Reference") (OtherBodyIndex :type Integer) (bFromSweep :type Boolean) (SweepResult :type "HitResult Structure (by ref)"))
  (if (`self.ActorHasTag` OtherActor "Player")
    (`SkeletalMeshComponent.PlayAnimation` (`self.Mesh`) "/Game/RPGHeroSquad/Animation/RPGHero/Anim_Idle_RPGHero.Anim_Idle_RPGHero" true)
    (`self.K2_SetActorRotation` (`KismetMathLibrary.Conv_VectorToRotator` (- (`self.K2_GetActorLocation` (`GameplayStatics.GetPlayerPawn` 0)) (`self.K2_GetActorLocation`))))
    (`SceneComponent.SetVisibility` (`self.Widget`) true false)
    (`self.SetLifeSpan` 4.0)
    (bind _asjam_character (cast `JamCharacter` OtherActor))
    (`JamCharacter.StartGod` _asjam_character)))

(fn `UserConstructionScript`)