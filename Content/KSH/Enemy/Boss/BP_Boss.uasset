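; BP_Boss is the boss enemy Blueprint, implementing its melee, ranged and area attacks on top of a parent class.
; ExecuteAttack damages a pawn found by a forward sphere trace.
; RangeAttack and AOEAttack stop movement and play a montage; on completion they fire a fanned projectile volley or scatter BP_BossAOE actors at random navigable points nearby.
; CallOnRangeEnd follows the volley, while CallOnAOEEnd runs after every AOE spawn.
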(event `self.ExecuteAttack`
  (`parent.ExecuteAttack`)
  (bind (_outhit _returnvalue) (`KismetSystemLibrary.SphereTraceSingleForObjects` (`self.K2_GetActorLocation`) (+ (`self.K2_GetActorLocation`) (* (`self.GetActorForwardVector`) 600.0)) 150.0 (`|MakeArray` "ObjectTypeQuery3" :!type "EObjectTypeQuery Enum")))
  (if _returnvalue
    (`GameplayStatics.ApplyDamage` (`.HitActor` (`GameplayStatics.BreakHitResult` _outhit)) 25.0)))

(event `RangeAttack`
  (`MovementComponent.StopMovementImmediately` (`self.CharacterMovement`))
  (`|PlayMontage` (`self.Mesh`) "/Game/LittleDragons/Animations/In_Place/AM_Boss_RangeAttack.AM_Boss_RangeAttack"
    (:`OnCompleted`
      (for _index (range 3)
        (bind _returnvalue (`|SpawnActorFromClass` "/Game/KSH/Enemy/Boss/BP_Projectile_Boss.BP_Projectile_Boss_C" (`self.GetTransform`) "AlwaysSpawn" "MultiplyWithRoot" null null))
        (set `MovementComponent.Velocity` (* (`KismetMathLibrary.GreaterGreater_VectorRotator` (`self.GetActorForwardVector`) (`KismetMathLibrary.MakeRotator` 0.0 0.0 (`KismetMathLibrary.Conv_IntToDouble` (* (- _index 1) 30)))) 1000.0) (`/Game/KSH/BP_ProjectileBase.ProjectileMovement` _returnvalue)))
      (`self.OnRangeEnd`))))

(event `AOEAttack`
  (`MovementComponent.StopMovementImmediately` (`self.CharacterMovement`))
  (`|PlayMontage` (`self.Mesh`) "/Game/LittleDragons/Animations/Common/AM_Boss_AOE.AM_Boss_AOE"
    (:`OnCompleted`
      (for _ (range 10)
        (bind _randomlocation (`NavigationSystemV1.K2_GetRandomLocationInNavigableRadius` (`self.K2_GetActorLocation`) 1500.0 null null))
        (`|SpawnActorFromClass` "/Game/KSH/Enemy/Boss/BP_BossAOE.BP_BossAOE_C" (`KismetMathLibrary.MakeTransform` _randomlocation) "AlwaysSpawn" "MultiplyWithRoot" null null)
        (`self.OnAOEEnd`)))))

(fn `UserConstructionScript`
  (`parent.UserConstructionScript`))