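; BP_ChestMonster is a chest monster enemy Blueprint that overrides the inherited ExecuteAttack event with a knockback strike.
; After calling the parent attack, it sphere-traces a short distance along its forward vector for Pawn objects.
; A hit actor takes fixed damage and, if it is a Character, is launched horizontally away from the monster with both XY and Z velocity overridden.
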(event `self.ExecuteAttack`
  (`parent.ExecuteAttack`)
  (bind (_outhit _returnvalue) (`KismetSystemLibrary.SphereTraceSingleForObjects` (`self.K2_GetActorLocation`) (+ (`self.K2_GetActorLocation`) (* (`self.GetActorForwardVector`) 300.0)) 50.0 (`|MakeArray` "ObjectTypeQuery3" :!type "EObjectTypeQuery Enum")))
  (if _returnvalue
    (`GameplayStatics.ApplyDamage` (`.HitActor` (`GameplayStatics.BreakHitResult` _outhit)) 10.0)
    (bind `_as캐릭터` (cast `Character` (`.HitActor` (`GameplayStatics.BreakHitResult` _outhit))))
    (`self.LaunchCharacter` `_as캐릭터` (* (`KismetMathLibrary.Vector_Normal2D` (- (`self.K2_GetActorLocation` (`.HitActor` (`GameplayStatics.BreakHitResult` _outhit))) (`self.K2_GetActorLocation`))) 2000.0) true true)))

(fn `UserConstructionScript`
  (`parent.UserConstructionScript`))