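; BP_CactusAOE is a short-lived area-of-effect damage actor for the Cactus enemy.
; On BeginPlay it shows its Niagara effect and waits briefly, then runs a single sphere overlap for JamCharacter pawns around itself and applies damage to each hit.
; It destroys itself shortly afterward; overlap and tick events are unused.
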(event `self.ReceiveBeginPlay`
  (`SceneComponent.SetVisibility` (`self.Niagara`) true false)
  (`KismetSystemLibrary.Delay` 1.0)
  (bind _outactors (`KismetSystemLibrary.SphereOverlapActors` (`self.K2_GetActorLocation`) 300.0 (`|MakeArray` "ObjectTypeQuery3" :!type "EObjectTypeQuery Enum") "/Script/Jam.JamCharacter"))
  (for _array_element _outactors
    (`GameplayStatics.ApplyDamage` _array_element 15.0))
  (`KismetSystemLibrary.Delay` 0.5)
  (`self.K2_DestroyActor`))

(fn `UserConstructionScript`
  (`parent.UserConstructionScript`))