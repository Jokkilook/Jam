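; BP_Cactus is a cactus enemy Blueprint whose attack spawns an area-of-effect actor in front of it.
; It overrides ExecuteAttack, calling the parent, stopping character movement immediately, then spawning BP_CactusAOE a fixed distance along its forward vector.
; The spawn adjusts for collisions but always succeeds; BeginPlay, overlap, Tick and construction add no logic of their own.
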(event `self.ExecuteAttack`
  (`parent.ExecuteAttack`)
  (`MovementComponent.StopMovementImmediately` (`self.CharacterMovement`))
  (`|SpawnActorFromClass` "/Game/KSH/Enemy/Cactus/BP_CactusAOE.BP_CactusAOE_C" (`KismetMathLibrary.MakeTransform` (+ (`self.K2_GetActorLocation`) (* (`self.GetActorForwardVector`) 500.0))) "AdjustIfPossibleButAlwaysSpawn" "MultiplyWithRoot" null null))

(fn `UserConstructionScript`
  (`parent.UserConstructionScript`))